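; One-shot explosion actor that knocks nearby NetPlayer characters away when it spawns, without applying damage.
; On BeginPlay it checks every NetPlayer's distance, switches those inside ExplosionRadius to Falling and adds velocity directly.
; The boost combines amplified horizontal momentum, a fixed upward lift and a radial push with quadratic distance falloff.
; It then destroys itself and spawns an explosion particle effect; the TANH falloff alternative is unused.
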(event EventBeginPlay
  (Variables|Default|SetLocationSelf (Transformation|GetActorLocation))
  (bind _outactors (Actor|GetAllActorsOfClass "/Script/PK.NetPlayer"))
  (for _array_element _outactors
    (Variables|Default|SetPlayerActor _array_element)
    (bind _output_get (Variables|Default|SetArg (Transformation|GetDistanceTo (Variables|Default|GetPlayerActor) self)))
    (Development|PrintString (Utilities|String|ToString(Float) _output_get))
    (if (< (Transformation|GetDistanceTo (Variables|Default|GetPlayerActor) self) (Variables|Default|GetExplosionRadius))
      (Pawn|Components|CharacterMovement|SetMovementMode (Variables|/Script/Engine.Character|GetCharacterMovement (Variables|Default|GetPlayerActor)) "MOVE_Falling" 0)
      (Variables|/Script/Engine.MovementComponent|SetVelocity (Variables|/Script/Engine.Character|GetCharacterMovement (Variables|Default|GetPlayerActor)) (+ (+ (Variables|/Script/Engine.MovementComponent|GetVelocity (Variables|/Script/Engine.Character|GetCharacterMovement (Variables|Default|GetPlayerActor))) (* (Math|Vector|MakeVector (* (.X (Math|Vector|BreakVector (Variables|/Script/Engine.MovementComponent|GetVelocity (Variables|/Script/Engine.Character|GetCharacterMovement (Variables|Default|GetPlayerActor))))) 0.5) (* (.Y (Math|Vector|BreakVector (Variables|/Script/Engine.MovementComponent|GetVelocity (Variables|/Script/Engine.Character|GetCharacterMovement (Variables|Default|GetPlayerActor))))) 0.5) 1e+02) 1.0)) (* (Class|KismetMathLibrary|GetDirectionVector (Variables|Default|GetLocationSelf) (Transformation|GetActorLocation (Variables|Default|GetPlayerActor))) (* (- 1.0 (Math|Float|Power (/ (Variables|Default|GetArg) (Variables|Default|GetExplosionRadius)) 2.0)) 1.3e+03))))))
  (Actor|DestroyActor)
  (Effects|SpawnEmitteratLocation "/Game/Particles/Explosion_old.Explosion_old" (Variables|Default|GetLocationSelf)))

(event EventActorBeginOverlap
  (params (OtherActor :type Actor%20Object%20Reference)))

(event EventTick
  (params (DeltaSeconds :type Float%20%28single-precision%29)))

(fn ConstructionScript)